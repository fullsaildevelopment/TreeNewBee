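; ImpSword_Bp is an imp sword gear actor with an early prototype of a blade damage volume.
; On BeginPlay it runs one box trace on the Visibility channel between two offsets along its up vector, sized by a damage extent variable.
; The trace is drawn for debugging, and its result is unused, so no damage is applied; Tick, overlap and construction are empty.
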(event EventBeginPlay
  (bind _returnvalue (Transformation|GetActorLocation))
  (Collision|BoxTraceByChannel (+ (* (Transformation|GetActorUpVector) (Variables|Default|GetDamageEdgeOffset_start)) _returnvalue) (+ _returnvalue (* (Transformation|GetActorUpVector) (Variables|Default|GetDamageEdgeOffset_end))) (Variables|Default|GetDamageVolumnExtend) "0, 0, 0" "TraceTypeQuery1" false 0 "ForDuration" true "(R=1.000000,G=0.000000,B=0.000000,A=1.000000)" "(R=0.000000,G=1.000000,B=0.000000,A=1.000000)" 6e+01))

(event Collision|EventActorBeginOverlap
  (params (OtherActor :type Actor%20Object%20Reference)))

(event EventTick
  (params (DeltaSeconds :type Float%20%28single-precision%29)))

(fn ConstructionScript)