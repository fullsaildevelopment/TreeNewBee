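; Lobby game mode for The Last Bastion that tracks joining player controllers and reads max connections and lobby name from the game instance.
; Map setting changes and rebuilt player lists are pushed to every LobbyPC_Bp.
; RespawnPlayer spawns a character at the first PlayerStart and refreshes everyone, though its call after login is disconnected.
; LaunchGame server-travels to GameMap, and SwapCharacter is an empty stub.
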(event Custom|SwapCharacter
  (params (PlayerController :type Player%20Controller%20Object%20Reference) (CharacterClass :type Character%20Class%20Reference) (ChangeStatus :type Boolean)))

(event Custom|SeverUpdateGameSettings
  (params (MapImage :type Texture%202D%20Object%20Reference) (MapName :type Text) (MapTime :type Text) (MapID :type Integer))
  ;[1 1 1] Server has madchanges, tell each clients to update
  (Variables|Default|SetGM_Map%20Image MapImage)
  (Variables|Default|SetGM_MapName MapName)
  (Variables|Default|SetGM_Map_Time MapTime)
  (Variables|Default|SetGM_MapID MapID)
  (for _array_element (Variables|ServerSettings|GetAllPlayerControllers_0)
    (bind _aslobby_pc_bp (Utilities|Casting|CastToLobbyPC_Bp _array_element))
    (Default|UpdateLobbySettings _aslobby_pc_bp (Variables|Default|GetGM_Map%20Image) (Variables|Default|GetGM_MapName) (Variables|Default|GetGM_Map_Time))))

(event Custom|Launch%20Game
  (Development|ExecuteConsoleCommand "servertravel/Game/Maps/GameMap" (Game|GetPlayerController 0)))

(event Custom|EveryOne%20Update
  (bind _allplayercontrollers_0 (Variables|ServerSettings|GetAllPlayerControllers_0))
  ;[1 1 1] Update Everyone's player info mation after a new play comes in
  (bind _output_get (Variables|Default|SetcurrentPlayer (Utilities|Array|Length (Variables|ServerSettings|GetAllPlayerControllers_0))))
  (if (> _output_get 0)
    (Utilities|Array|Clear (Variables|Default|GetConnectedPlayers))
    (for _array_element _allplayercontrollers_0
      (bind _aslobby_pc_bp (Utilities|Casting|CastToLobbyPC_Bp _array_element))
      (Utilities|Array|Add (Variables|Default|GetConnectedPlayers) (Variables|/Game/Blueprints/PC/LobbyPC_BP.LobbyPC_Bp_C|GetplayerSettings _aslobby_pc_bp))
      (Default|UpdateNumOfPlayers _aslobby_pc_bp (Variables|Default|GetcurrentPlayer) (Variables|Default|Getmax%20players)))
    (for _array_element_2 _allplayercontrollers_0
      (bind _aslobby_pc_bp_2 (Utilities|Casting|CastToLobbyPC_Bp _array_element_2))
      (Default|AddPlayerInfo _aslobby_pc_bp_2 (Variables|Default|GetConnectedPlayers)))))

(event Custom|RespawnPlayer
  (params (playerController :type Player%20Controller%20Object%20Reference))
  (bind _returnvalue (Pawn|GetControlledPawn playerController))
  ;[1 1 1] Spawn player as base character when arriving to the lobby
  (Utilities|IsValid _returnvalue
    (:Is%20Valid
      (Actor|DestroyActor _returnvalue))
    (:Is%20Not%20Valid
      _))
  (bind _returnvalue_2 (Game|SpawnActorfromClass "/Script/Engine.Character" (Transformation|GetActorTransform (Utilities|Array|Get(acopy) (Variables|Default|GetPlayerStartsPoint))) "Undefined" 0 0))
  (Pawn|Possess playerController _returnvalue_2)
  (CallFunction|EveryOneUpdate))

(event EventPostLogin
  (params (NewPlayer :type Player%20Controller%20Object%20Reference))
  ;[1 1 1] Post Log in
  (Networking|SwitchHasAuthority
    (:Authority
      (Utilities|Array|Add (Variables|ServerSettings|GetAllPlayerControllers_0) NewPlayer)
      (bind _outactors (Actor|GetAllActorsOfClass "/Script/Engine.PlayerStart"))
      (Variables|Default|SetPlayerStartsPoint _outactors)
      (bind _asgi_the_last_bastion_bp (Utilities|Casting|CastToGI_TheLastBastion_BP (Game|GetGameInstance)))
      (Variables|Default|Setmax%20players (Class|GItheLastBastion|GetMaxConnection _asgi_the_last_bastion_bp))
      (Variables|Default|SetLobbyName_0 (Class|GItheLastBastion|GetLobbyName _asgi_the_last_bastion_bp))
      (bind _aslobby_pc_bp (Utilities|Casting|CastToLobbyPC_Bp NewPlayer)))))

(fn ConstructionScript)