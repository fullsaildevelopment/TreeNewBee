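; Builder hero character that carries a weapon actor and fires it on player input.
; On BeginPlay it spawns a Lan_T0_CB_Bp, attaches it to the mesh's TestSocket with relative rules, stores it as CB and takes ownership of it.
; The Attack input press calls Fire on CB.
; Landing reports a noise event at the actor's location to debug AI hearing perception.
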(event EventOnLanded
  (params (Hit :type Hit%20Result%20Structure%20%28by%20ref%29))
  ;[1 1 1] Debug AI Hearing Perception
  (Class|AISenseHearing|ReportNoiseEvent (Transformation|GetActorLocation) 1.0 self 0.0 "None"))

(event EventBeginPlay
  (bind _returnvalue (Game|SpawnActorfromClass "/Game/Blueprints/Gears/Lan/Lan_T0_CB_Bp.Lan_T0_CB_Bp_C" (Math|Conversions|ToTransform(Vector) (Math|Vector|MakeVector 0.0 0.0 0.0)) "AlwaysSpawn" 0 0))
  (Transformation|AttachComponentToComponent _returnvalue (Variables|Character|GetMesh) "TestSocket" "KeepRelative" "KeepRelative" "KeepRelative" true)
  (bind _output_get (Variables|Default|SetCB _returnvalue))
  (Actor|SetOwner _output_get self))

(event Input|ActionEvents|InputActionAttack
  (params (Key :type Key%20Structure))
  (:Pressed
    (Class|RangeWeapon|Fire (Variables|Default|GetCB))))

(fn ConstructionScript)