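; Single-player hero character Blueprint that drops the character into a ragdoll when the Ragdoll input is pressed.
; The press enables mesh collision and physics below a named bone, sets IsRagDoll, notifies the anim instance and disables player input.
; Unconnected nodes hold unused logic for exiting ragdoll by reattaching the mesh, and for moving the capsule to follow the bone, so ragdoll is one-way here.
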(event EventTick
  (params (DeltaSeconds :type Float%20%28single-precision%29)))

(event Input|ActionEvents|InputActionRagdoll
  (params (Key :type Key%20Structure))
  (bind _newvar_0 (Variables|Default|GetNewVar_0))
  (bind _mesh (Variables|Character|GetMesh))
  (:Pressed
    (Collision|SetCollisionResponsetoChannel _mesh "ECC_WorldStatic" "ECR_Block")
    (Collision|SetCollisionEnabled _mesh "QueryAndPhysics")
    (Class|SkeletalMeshComponent|SetAllBodiesBelowPhysicsBlendWeight (Variables|Character|GetMesh) _newvar_0 1.0 false true)
    (Class|SkeletalMeshComponent|SetAllBodiesBelowSimulatePhysics _mesh _newvar_0 true true)
    (Variables|Default|SetbIsRagDoll true)
    (Class|BaseAnimInstance|AnimInstanceResetonRagDoll (Variables|Default|GetmAnimInstanceRef))
    (Input|DisableInput (Game|GetPlayerController 0))))

(fn ConstructionScript)